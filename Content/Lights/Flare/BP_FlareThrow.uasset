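; BP_FlareThrow is a thrown flare with a point light, Niagara effect and audio.
; It flies on projectile movement, then switches its static mesh to physics simulation on the first bounce.
; Thirty seconds after spawn it sets the light intensity to zero, deactivates the effect and stops the sound.
; A disconnected delay, meant to prevent wall clipping, is left unused.
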(event OnProjectileBounce(ProjectileMovement)
  (params (ImpactResult :type Hit%20Result%20Structure%20%28by%20ref%29) (ImpactVelocity :type Vector%20%28by%20ref%29 :default "0, 0, 0"))
  ;[1 0.4453 0] Convert from projectile to SM physics on Hit
  (Physics|SetSimulatePhysics (Variables|Default|GetStaticMesh) true))

(event EventBeginPlay
  (Utilities|FlowControl|Delay 3e+01)
  (Rendering|Components|Light|SetIntensity (Variables|Default|GetPointLight) 0.0)
  (Components|Activation|Deactivate (Variables|Default|GetNiagara1))
  (Audio|Components|Audio|Stop (Variables|Default|GetAudio)))

(fn ConstructionScript)