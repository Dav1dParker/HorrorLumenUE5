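; BP_ChemLightHand is a green chem light projectile whose neon glow fades over time.
; On BeginPlay it creates a dynamic Neon material on the mesh and starts a looping timer that steadily lowers the NeonEmission parameter, clearing itself once emission is used up.
; On the first projectile bounce, the static mesh switches to simulated physics.
; A delay meant to prevent wall clipping is left disconnected.
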(event OnProjectileBounce(ProjectileMovement)
  (params (ImpactResult :type Hit%20Result%20Structure%20%28by%20ref%29) (ImpactVelocity :type Vector%20%28by%20ref%29 :default "0, 0, 0"))
  ;[1 0.4453 0] Convert from projectile to SM physics on Hit
  (Physics|SetSimulatePhysics (Variables|Default|GetChemLightGreen) true))

(event Custom|Attenuation
  (bind _output_get (Variables|Default|SetEmission (- (Variables|Default|GetEmission) 1e+01)))
  (Rendering|Material|SetScalarParameterValue (Variables|Default|GetNewMaterial) "NeonEmission" _output_get :!class /Script/Engine.MaterialInstanceDynamic)
  (if (not (> (Variables|Default|GetEmission) 0.0))
    (Utilities|Time|ClearandInvalidateTimerbyHandle (stale EventBeginPlay _returnvalue_2))))

(event EventBeginPlay
  (bind _returnvalue (Rendering|Material|CreateDynamicMaterialInstance (Variables|Default|GetChemLightGreen) 1 "/Game/Lights/ChemStick/Neon.Neon" "None" :!class /Script/Engine.PrimitiveComponent))
  (Variables|Default|SetNewMaterial _returnvalue)
  (bind _returnvalue_2 (Utilities|Time|SetTimerbyEvent (delegate Custom|Attenuation) 0.5 true)))

(fn ConstructionScript)