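; BP_Enemy is an enemy that distorts the screen as the player nears and signals death on contact.
; While GrainZone is overlapped, Tick drives PostProcessVolume film grain inversely with distance, jumping to heavy grain and Intensity at close range.
; Leaving the zone stops Tick and clears the effect.
; A mesh hit broadcasts CharacterDiedMessage to all BI_Observer actors, while its CharacterDied event stops Tick.
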(event OnComponentBeginOverlap(GrainZone)
  (params (OverlappedComponent :type Primitive%20Component%20Object%20Reference) (OtherActor :type Actor%20Object%20Reference) (OtherComp :type Primitive%20Component%20Object%20Reference) (OtherBodyIndex :type Integer) (bFromSweep :type Boolean) (SweepResult :type Hit%20Result%20Structure%20%28by%20ref%29))
  (Actor|Tick|SetActorTickEnabled true))

(event OnComponentEndOverlap(GrainZone)
  (params (OverlappedComponent :type Primitive%20Component%20Object%20Reference) (OtherActor :type Actor%20Object%20Reference) (OtherComp :type Primitive%20Component%20Object%20Reference) (OtherBodyIndex :type Integer))
  ;[1 0.8906 0] Turn off when too far
  (Actor|Tick|SetActorTickEnabled false)
  (bind _returnvalue (Actor|GetActorOfClass "/Script/Engine.PostProcessVolume"))
  (Variables|/Script/Engine.PostProcessVolume|SetSettings _returnvalue (Utilities|Struct|MakePostProcessSettings 0.0)))

(event OnComponentHit(SM_Enemy)
  (params (HitComponent :type Primitive%20Component%20Object%20Reference) (OtherActor :type Actor%20Object%20Reference) (OtherComp :type Primitive%20Component%20Object%20Reference) (NormalImpulse :type Vector :default "0, 0, 0") (Hit :type Hit%20Result%20Structure%20%28by%20ref%29))
  ;[1 0 0.1172] Character hit enemy
  (bind _outactors (Actor|GetAllActorswithInterface "/Game/Logic/BI_Observer.BI_Observer_C"))
  (for _array_element _outactors
    (Class|BIObserver|CharacterDied(Message) _array_element)))

(event EventTick
  (params (DeltaSeconds :type Float%20%28single-precision%29))
  (bind _returnvalue (Game|GetPlayerCharacter 0))
  (bind _self self)
  (bind _returnvalue_2 (Transformation|GetDistanceTo _returnvalue _self))
  ;[1 0.07031 0] Post effects
  (bind _returnvalue_3 (Actor|GetActorOfClass "/Script/Engine.PostProcessVolume"))
  (if (> _returnvalue_2 2e+02)
    (Variables|/Script/Engine.PostProcessVolume|SetSettings _returnvalue_3 (Utilities|Struct|MakePostProcessSettings 0.0 (/ 5e+02 _returnvalue_2)))
    (else
      ;;[1 0 0.9609] Too close
      (Variables|/Script/Engine.PostProcessVolume|SetSettings _returnvalue_3 (Utilities|Struct|MakePostProcessSettings 2e+01 5e+01)))))

(event EventCharacterDied
  ;[0 0.8125 1] Player died
  (Actor|Tick|SetActorTickEnabled false))

(fn ConstructionScript)