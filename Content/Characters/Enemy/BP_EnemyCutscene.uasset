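; BP_EnemyCutscene is an enemy Blueprint, named for cutscene use, whose gameplay events are all empty.
; Tick, mesh hit, GrainZone overlap and CharacterDied handlers do nothing, as do the construction script and PassPlayerSettings.
; Disconnected leftover nodes would scale post-process film grain by player distance to BP_Enemy actors, toggle ticking and broadcast death to BPI_Observer actors, but none of them run.
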(event OnComponentBeginOverlap(GrainZone)
  (params (OverlappedComponent :type Primitive%20Component%20Object%20Reference) (OtherActor :type Actor%20Object%20Reference) (OtherComp :type Primitive%20Component%20Object%20Reference) (OtherBodyIndex :type Integer) (bFromSweep :type Boolean) (SweepResult :type Hit%20Result%20Structure%20%28by%20ref%29)))

(event OnComponentEndOverlap(GrainZone)
  (params (OverlappedComponent :type Primitive%20Component%20Object%20Reference) (OtherActor :type Actor%20Object%20Reference) (OtherComp :type Primitive%20Component%20Object%20Reference) (OtherBodyIndex :type Integer))
  ;[1 0.8906 0] Turn off when too far
)

(event OnComponentHit(SM_Enemy)
  (params (HitComponent :type Primitive%20Component%20Object%20Reference) (OtherActor :type Actor%20Object%20Reference) (OtherComp :type Primitive%20Component%20Object%20Reference) (NormalImpulse :type Vector :default "0, 0, 0") (Hit :type Hit%20Result%20Structure%20%28by%20ref%29))
  ;[1 0 0.1172] Character hit enemy
)

(event EventTick
  (params (DeltaSeconds :type Float%20%28single-precision%29))
  ;[1 0.07031 0] Post effects
  ;;[0 0.3672 1] Bad
)

(event EventCharacterDied
  ;[0 0.8125 1] Player died
)

(fn ConstructionScript)

(fn PassPlayerSettings
  (params (GGraphicsIndexIn :type Integer) (GWindowModeIn :type EWindowMode%20Enum :default "Fullscreen") (GVsyncIn :type Boolean) (GResolutionIndexIn :type Integer) (GFSRQualityIn :type Integer) (GFrameGenIn :type ECheckBoxState%20Enum :default "Unchecked") (GLumenIndexIn :type Integer))
  (return))