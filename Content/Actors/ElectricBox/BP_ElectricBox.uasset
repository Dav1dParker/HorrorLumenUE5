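; BP_ElectricBox is an interactable electric box that triggers the basement light event and advances the game state.
; On InteractE it sets IsBroken so it fires only once, calls TurnOn on BP_BasementLight, then sets the first-person character's GameState and calls UpdateInGameState.
; Both actors are found with GetActorOfClass.
; A disconnected, never-run chain holds an inline version of a light sequence with buzz, bulb break and sparks.
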(event EventBeginPlay)

(event Collision|EventActorBeginOverlap
  (params (OtherActor :type Actor%20Object%20Reference)))

(event EventTick
  (params (DeltaSeconds :type Float%20%28single-precision%29)))

(event EventInteractE
  (params (HitComponent :type Primitive%20Component%20Object%20Reference))
  (if (not (Variables|Default|GetIsBroken))
    (Variables|Default|SetIsBroken true)
    (bind _returnvalue (Actor|GetActorOfClass "/Game/Actors/BasementLight/BP_BasementLight.BP_BasementLight_C"))
    (Default|Turnon _returnvalue)
    (bind _returnvalue_2 (Actor|GetActorOfClass "/Game/FirstPerson/Blueprints/BP_FirstPersonCharacter.BP_FirstPersonCharacter_C"))
    (Variables|/Game/FirstPerson/Blueprints/BP_FirstPersonCharacter.BP_FirstPersonCharacter_C|SetGameState _returnvalue_2 2)
    (Default|UpdateinGameState _returnvalue_2)))

(fn ConstructionScript)