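; BP_Door is an interactable hinged door that can require a key and may slam shut by itself.
; InteractE toggles it, checking the player character's HaveKey for locked doors and showing a subtitle hint when it is missing.
; Timelines lerp the door mesh's yaw to open or close it, with matching sounds.
; The open timeline's update also runs a delayed coin flip that can trigger DoorShut, snapping the door closed with a slam sound.
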(event Custom|OpenDoor
  (bind _dooraudio (Variables|Default|GetDoorAudio))
  ;[0 1 0.4375] Open
  (Audio|Components|Audio|SetSound _dooraudio "/Game/Audio/Cues/FX/C_DoorOpen_Cue.C_DoorOpen_Cue")
  (Audio|Components|Audio|Play _dooraudio 0.0)
  (bind _doorfloat (Timeline|Open%20door%20timeline PlayFromStart)
    (:Update
      (Transformation|SetRelativeRotation (Variables|Default|GetDoorWithoutFrame_Apt_01) (Math|Rotator|MakeRotator 0.0 0.0 (Math|Float|Lerp 0.0 9e+01 _doorfloat)) false false)
      (Variables|Default|SetIsOpen true)
      (Utilities|FlowControl|Delay 2e+01)
      (if (and (Math|Random|RandomBool) (Variables|Default|GetIsOpen))
        (CallFunction|DoorShut)
        (Variables|Default|SetIsOpen false)))))

(event Custom|CloseDoor
  (bind _dooraudio (Variables|Default|GetDoorAudio))
  ;[0.1016 1 0] Close
  (Audio|Components|Audio|SetSound _dooraudio "/Game/Audio/Cues/FX/C_DoorClose_Cue.C_DoorClose_Cue")
  (Audio|Components|Audio|Play _dooraudio 0.0)
  (bind _doorfloat (Timeline|Timeline PlayFromStart)
    (:Update
      (Transformation|SetRelativeRotation (Variables|Default|GetDoorWithoutFrame_Apt_01) (Math|Rotator|MakeRotator 0.0 0.0 (Math|Float|Lerp 9e+01 0.0 _doorfloat)) false false)
      (Variables|Default|SetIsOpen false))))

(event Custom|DoorShut
  (bind _dooraudio (Variables|Default|GetDoorAudio))
  ;[0.1719 1 0] DoorShut
  (Variables|/Script/Engine.AudioComponent|SetVolumeMultiplier _dooraudio 4e+01)
  (Audio|Components|Audio|SetSound _dooraudio "/Game/Audio/Cues/FX/C_DoorShut.C_DoorShut")
  (Audio|Components|Audio|Play _dooraudio 0.0)
  (Transformation|SetRelativeRotation (Variables|Default|GetDoorWithoutFrame_Apt_01) "0, 0, 0" false false)
  (Audio|Components|Audio|SetVolumeMultiplier _dooraudio 3.0 :!class /Script/Engine.AudioComponent))

(event EventInteractE
  (params (HitComponent :type Primitive%20Component%20Object%20Reference))
  (if (Variables|Default|GetIsOpen)
    (CallFunction|CloseDoor)
    (elif (Variables|Default|GetKey%20Required)
      (bind _returnvalue (Actor|GetActorOfClass "/Game/FirstPerson/Blueprints/BP_FirstPersonCharacter.BP_FirstPersonCharacter_C"))
      (if (Variables|/Game/FirstPerson/Blueprints/BP_FirstPersonCharacter.BP_FirstPersonCharacter_C|GetHaveKey _returnvalue)
        (CallFunction|OpenDoor)
        (else
          (Variables|/Game/FirstPerson/Blueprints/BP_FirstPersonCharacter.BP_FirstPersonCharacter_C|SetInText _returnvalue "Door is locked. I need to find a key. 
It has to be somewhere here")
          (Variables|/Game/FirstPerson/Blueprints/BP_FirstPersonCharacter.BP_FirstPersonCharacter_C|SetSubsDelay _returnvalue 6.0)
          (Default|CallSubtitles _returnvalue)))
      (else
        (CallFunction|OpenDoor)))))

(fn ConstructionScript)