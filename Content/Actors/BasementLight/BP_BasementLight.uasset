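; BP_BasementLight is a basement fluorescent light that switches on noisily, then breaks in a burst of sparks.
; The Turnon event plays a buzzing sound and lights the lamp, then after a delay swaps to a loud bulb-break sound and kills the intensity.
; A looping timer repeatedly calls Sparks to activate four spark effect components until it is paused after a second delay.
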(event Custom|Turn%20on
  (bind _sound (Variables|Default|GetSound))
  (bind _sound_2 (Variables|Default|GetSound))
  (Audio|Components|Audio|SetSound _sound "/Game/Audio/Source/676841__brokkolix__noisy-old-fluorescent-light.676841__brokkolix__noisy-old-fluorescent-light")
  (Audio|Components|Audio|Play _sound 0.0)
  (Rendering|Components|Light|SetIntensity (Variables|Default|GetLight) 31407.029297)
  (Utilities|FlowControl|Delay 4.0)
  (Audio|Components|Audio|SetSound _sound_2 "/Game/Audio/Source/558969__sandb1ns__fluorescent-lightbulb-break.558969__sandb1ns__fluorescent-lightbulb-break")
  (Audio|Components|Audio|SetVolumeMultiplier _sound_2 7.0 :!class /Script/Engine.AudioComponent)
  (Audio|Components|Audio|Play _sound_2 0.0)
  (Rendering|Components|Light|SetIntensity (Variables|Default|GetLight) 0.0)
  (bind _returnvalue (Utilities|Time|SetTimerbyEvent (delegate Custom|Sparks) 0.1 true))
  (Utilities|FlowControl|Delay 4.0)
  (Utilities|Time|PauseTimerbyHandle _returnvalue))

(event Custom|Sparks
  (Components|Activation|SetActive (.NS_Spark2 (|CollapseGraph)) true false))

(event EventBeginPlay)

(event Collision|EventActorBeginOverlap
  (params (OtherActor :type Actor%20Object%20Reference)))

(event EventTick
  (params (DeltaSeconds :type Float%20%28single-precision%29)))

(fn ConstructionScript)