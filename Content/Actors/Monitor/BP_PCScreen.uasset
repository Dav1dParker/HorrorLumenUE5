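; BP_PCScreen is an interactable PC screen that runs a loading sequence with video and voice cues.
; InteractE plays the loading-started sound on VoiceLoading and starts the progress bar video on TVMediaPlayer.
; A fixed delay of about a minute, rather than a media-end event, triggers the loading-complete sound.
; BeginPlay only runs a short delay with nothing after it.
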(event EventBeginPlay
  (Utilities|FlowControl|Delay 5.0))

(event EventInteractE
  (params (HitComponent :type Primitive%20Component%20Object%20Reference))
  (bind _voiceloading (Variables|Default|GetVoiceLoading))
  (bind _voiceloading_2 (Variables|Default|GetVoiceLoading))
  (Audio|Components|Audio|SetSound _voiceloading_2 "/Game/Audio/Source/C_Loading_started.C_Loading_started")
  (Audio|Components|Audio|Play _voiceloading_2 0.0)
  (Media|MediaPlayer|OpenSource (Variables|Default|GetTV%20Media%20Player) "/Game/Movies/FMS_ProgressBar.FMS_ProgressBar")
  (Media|MediaPlayer|Play (Variables|Default|GetTV%20Media%20Player) :!class /Script/MediaAssets.MediaPlayer)
  (Utilities|FlowControl|Delay 66.0)
  (Audio|Components|Audio|SetSound _voiceloading "/Game/Audio/Cues/FX/C_Loading_completeV2_Cue.C_Loading_completeV2_Cue")
  (Audio|Components|Audio|Play _voiceloading 0.0))

(fn ConstructionScript)